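; BP_Player is the player Blueprint, moved by input across the world Y-Z plane.
; BeginPlay adds the IMC_PlayerInput Enhanced Input mapping context, and the IA_Horizontal and IA_Vertical Triggered events store their axis values.
; Tick normalizes those values into a direction and moves the actor by MoveSpeed times delta time, setting its location directly without sweep collision.
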(event Input|EnhancedActionEvents|EnhancedInputActionIA_Horizontal
  (params (ActionValue :type Float%20%28double-precision%29) (ElapsedSeconds :type Float%20%28double-precision%29) (TriggeredSeconds :type Float%20%28double-precision%29) (InputAction :type Input%20Action%20Object%20Reference :default "/Game/Input/IA_Horizontal.IA_Horizontal"))
  (:Triggered
    (Variables|Default|SetHorizontal ActionValue)))

(event Input|EnhancedActionEvents|EnhancedInputActionIA_Vertical
  (params (ActionValue :type Float%20%28double-precision%29) (ElapsedSeconds :type Float%20%28double-precision%29) (TriggeredSeconds :type Float%20%28double-precision%29) (InputAction :type Input%20Action%20Object%20Reference :default "/Game/Input/IA_Vertical.IA_Vertical"))
  (:Triggered
    (Variables|Default|SetVertical ActionValue)))

(event EventBeginPlay
  (Input|AddMappingContext (PlayerController|LocalPlayerSubsystems|GetEnhancedInputLocalPlayerSubsystem (Game|GetPlayerController 0)) "/Game/Input/IMC_PlayerInput.IMC_PlayerInput" 0 "(bIgnoreAllPressedKeysUntilRelease=True,bForceImmediately=False,bNotifyUserSettings=False)"))

(event Collision|EventActorBeginOverlap
  (params (OtherActor :type Actor%20Object%20Reference)))

(event EventTick
  (params (DeltaSeconds :type Float%20%28single-precision%29))
  ;[1 1 1] 이동 P = p0+vt
  (Transformation|SetActorLocation (+ (Transformation|GetActorLocation) (* (* (Math|Vector|Normalize (Math|Vector|MakeVector 0.0 (Variables|Default|GetHorizontal) (Variables|Default|GetVertical))) (Variables|Default|GetMoveSpeed)) DeltaSeconds)) false false))

(fn ConstructionScript)